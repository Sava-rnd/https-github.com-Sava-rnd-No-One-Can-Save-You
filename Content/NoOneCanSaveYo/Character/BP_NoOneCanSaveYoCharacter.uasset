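; Player character Blueprint for NoOneCanSaveYo that handles jumping and interacting with nearby objects through Enhanced Input actions.
; Capsule overlaps store an actor implementing BPI_Interactable as CurrentInteract only when none is held, and clear it when that actor's overlap ends.
; The interact action sends InteractMessage to the stored actor if it is still valid.
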(event OnComponentBeginOverlap(CapsuleComponent)
  (params (OverlappedComponent :type Primitive%20Component%20Object%20Reference) (OtherActor :type Actor%20Object%20Reference) (OtherComp :type Primitive%20Component%20Object%20Reference) (OtherBodyIndex :type Integer) (bFromSweep :type Boolean) (SweepResult :type Hit%20Result%20Structure%20%28by%20ref%29))
  (if (Utilities|DoesObjectImplementInterface OtherActor "/Game/NoOneCanSaveYo/Blueprints/BPI_Interactable.BPI_Interactable_C")
    (Utilities|IsValid (Variables|Default|GetCurrentInteract)
      (:Is%20Not%20Valid
        (Variables|Default|SetCurrentInteract OtherActor)))))

(event OnComponentEndOverlap(CapsuleComponent)
  (params (OverlappedComponent :type Primitive%20Component%20Object%20Reference) (OtherActor :type Actor%20Object%20Reference) (OtherComp :type Primitive%20Component%20Object%20Reference) (OtherBodyIndex :type Integer))
  (if (== OtherActor (Variables|Default|GetCurrentInteract))
    (Variables|Default|SetCurrentInteract 0)))

(event Input|EnhancedActionEvents|EnhancedInputActionIA_NoOneCanSaveYoJump
  (params (ActionValue :type Boolean) (ElapsedSeconds :type Float%20%28double-precision%29) (TriggeredSeconds :type Float%20%28double-precision%29) (InputAction :type Input%20Action%20Object%20Reference :default "/Game/NoOneCanSaveYo/Core/EnhancedInput/Action/IA_NoOneCanSaveYoJump.IA_NoOneCanSaveYoJump"))
  (:Triggered
    (Character|Jump))
  (:Completed
    (Character|StopJumping)))

(event Input|EnhancedActionEvents|EnhancedInputActionIA_NoOneCanSaveYoInteract
  (params (ActionValue :type Boolean) (ElapsedSeconds :type Float%20%28double-precision%29) (TriggeredSeconds :type Float%20%28double-precision%29) (InputAction :type Input%20Action%20Object%20Reference :default "/Game/NoOneCanSaveYo/Core/EnhancedInput/Action/IA_NoOneCanSaveYoInteract.IA_NoOneCanSaveYoInteract"))
  (bind _currentinteract (Variables|Default|GetCurrentInteract))
  (Utilities|IsValid _currentinteract
    (:Is%20Valid
      (Class|BPIInteractable|Interact(Message) _currentinteract))))

(event EventBeginPlay)

(event Collision|EventActorBeginOverlap
  (params (OtherActor :type Actor%20Object%20Reference)))

(event EventTick
  (params (DeltaSeconds :type Float%20%28single-precision%29)))

(fn ConstructionScript)