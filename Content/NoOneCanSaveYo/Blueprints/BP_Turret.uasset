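; Turret actor that sweeps its mesh through a timeline-driven yaw patrol and switches to shooting when it detects the player character.
; Tick runs the Patrol/Shoot states, using a forward sphere trace for detection and interpolating yaw toward the player while shooting.
; A looping timer fires shots with sound, an explosion emitter and a line trace, whose hit result triggers nothing.
; Losing sight clears the timer and restarts patrol from the current rotation.
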(event Custom|StopPatrol
  (bind _rotatetrack (Timeline|Timeline Stop)
    (:Update
      (Transformation|SetWorldRotation (Variables|Default|GetSkeletalMesh) (Math|Rotator|Lerp(Rotator) (Variables|Default|GetCurrentRotation) (Variables|Default|GetTargetRotation) _rotatetrack) false false))
    (:Finished
      (switch Utilities|FlowControl|Switch|SwitchonETimelineDirection (Variables|Default|GetDirictionMove)
        (:Forward
          (Variables|Default|SetDirictionMove "Backward")
          (Variables|Default|SetTargetRotation (Variables|Default|GetStartRotation))
          (Variables|Default|SetCurrentRotation (Variables|Default|GetEndRotation)))
        (:Backward
          (Variables|Default|SetDirictionMove "Forward")
          (Variables|Default|SetCurrentRotation (Variables|Default|GetEndRotation))
          (Variables|Default|SetTargetRotation (Variables|Default|GetStartRotation))))
      (CallFunction|StartPatrol))))

(event Custom|StartPatrol
  (bind _rotatetrack (Timeline|Timeline PlayFromStart)
    (:Update
      (Transformation|SetWorldRotation (Variables|Default|GetSkeletalMesh) (Math|Rotator|Lerp(Rotator) (Variables|Default|GetCurrentRotation) (Variables|Default|GetTargetRotation) _rotatetrack) false false))
    (:Finished
      (switch Utilities|FlowControl|Switch|SwitchonETimelineDirection (Variables|Default|GetDirictionMove)
        (:Forward
          (Variables|Default|SetDirictionMove "Backward")
          (Variables|Default|SetTargetRotation (Variables|Default|GetStartRotation))
          (Variables|Default|SetCurrentRotation (Variables|Default|GetEndRotation)))
        (:Backward
          (Variables|Default|SetDirictionMove "Forward")
          (Variables|Default|SetCurrentRotation (Variables|Default|GetEndRotation))
          (Variables|Default|SetTargetRotation (Variables|Default|GetStartRotation))))
      (CallFunction|StartPatrol))))

(event Custom|StartShoot
  (bind _returnvalue (Utilities|Time|SetTimerbyEvent (delegate Custom|CallShootFunc) 1.0 true))
  (Variables|Default|SetShootTimer _returnvalue))

(event Custom|CallShootFunc
  (bind _bisshoot (CallFunction|Shoot))
  (if _bisshoot
    _))

(event EventTick
  (params (DeltaSeconds :type Float%20%28single-precision%29))
  (bind _skeletalmesh (Variables|Default|GetSkeletalMesh))
  (bind _returnvalue (Transformation|GetWorldRotation _skeletalmesh))
  (switch Utilities|FlowControl|Switch|SwitchonE_TurretStates (Variables|Default|GetCurrentState)
    (:NewEnumerator0
      (bind _bisplayerfind (CallFunction|PlayerSearch))
      (if _bisplayerfind
        (CallFunction|StopPatrol)
        (Variables|Default|SetCurrentState "NewEnumerator1")))
    (:NewEnumerator1
      (Transformation|SetWorldRotation _skeletalmesh (Math|Interpolation|RInterpTo (Math|Rotator|MakeRotator (.roll _returnvalue) (.pitch _returnvalue) (.yaw _returnvalue)) (Math|Rotator|MakeRotator (.roll _returnvalue) (.pitch _returnvalue) (- (.yaw (Math|Rotator|FindLookatRotation (Transformation|GetWorldLocation (Variables|Default|GetSkeletalMesh)) (Transformation|GetActorLocation (Game|GetPlayerCharacter 0)))) 9e+01)) (Utilities|Time|GetWorldDeltaSeconds) 0.0) false false)
      (Utilities|FlowControl|Sequence
        (:then_0
          (if (not (Variables|Default|GetbIsStartShoot))
            (CallFunction|StartShoot)
            (Variables|Default|SetbIsStartShoot true)))
        (:then_1
          (bind _bisplayerfind_2 (CallFunction|PlayerSearch))
          (if (not _bisplayerfind_2)
            (Utilities|Time|ClearandInvalidateTimerbyHandle (Variables|Default|GetShootTimer))
            (Variables|Default|SetCurrentState "NewEnumerator0")
            (Variables|Default|SetbIsStartShoot false)
            (CallFunction|StartPatrol)
            (Variables|Default|SetTargetRotation (Variables|Default|GetEndRotation))
            (Variables|Default|SetCurrentRotation (Transformation|GetWorldRotation (Variables|Default|GetSkeletalMesh)))
            (Variables|Default|SetDirictionMove "Forward")
            (CallFunction|StartPatrol)))))))

(event EventBeginPlay
  (bind _output_get (Variables|Default|SetStartRotation (Transformation|GetWorldRotation (Variables|Default|GetSkeletalMesh))))
  (Variables|Default|SetEndRotation (Math|Rotator|MakeRotator (.roll _output_get) (.pitch _output_get) (+ (.yaw _output_get) 1.8e+02)))
  (Variables|Default|SetCurrentRotation (Variables|Default|GetStartRotation))
  (Variables|Default|SetTargetRotation (Variables|Default|GetEndRotation))
  (CallFunction|StartPatrol))

(fn ConstructionScript)

(fn PlayerSearch
  (bind _scene (Variables|Default|GetScene))
  (bind _returnvalue (Transformation|GetWorldLocation _scene))
  (bind (_outhit _returnvalue_2) (Collision|SphereTraceByChannel _returnvalue (+ _returnvalue (* (Math|Vector|GetForwardVector _scene) (Variables|Default|GetSearchDistance))) 1e+01 "TraceTypeQuery3" false 0 "None"))
  (if _returnvalue_2
    (Utilities|Casting|CastToBP_NoOneCanSaveYoCharacter (.HitActor (Collision|BreakHitResult _outhit))
      (:then
        (return true))
      (:CastFailed
        (return false)))
    (else
      (return false))))

(fn Shoot
  (bind _scene (Variables|Default|GetScene))
  (bind _shootdistance (Variables|Default|GetShootDistance))
  (bind _returnvalue (Math|Vector|GetForwardVector _scene))
  (bind _returnvalue_2 (* _returnvalue _shootdistance))
  (bind (_outhit _returnvalue_3) (Collision|LineTraceByChannel (+ (Transformation|GetWorldLocation _scene) _returnvalue_2) _returnvalue_2 "TraceTypeQuery3" false 0 "None"))
  (Utilities|FlowControl|Sequence
    (:then_0
      (Audio|PlaySoundatLocation "/Game/NoOneCanSaveYo/Core/Audio/Звук_из_CS_1_6_рикошет__mp3cut_net_.Звук_из_CS_1_6_рикошет__mp3cut_net_" (Transformation|GetWorldLocation (Variables|Default|GetScene)) "0, 0, 0" 1.0 1.0 0.0 0 0 0 0)
      (Effects|SpawnEmitterAttached "/Game/StarterContent/Particles/P_Explosion.P_Explosion" (Variables|Default|GetScene) "None"))
    (:then_1
      (if _returnvalue_3
        (Utilities|Casting|CastToBP_NoOneCanSaveYoCharacter (.HitActor (Collision|BreakHitResult _outhit))
          (:then
            (return true))
          (:CastFailed
            (return false)))
        (else
          (return false))))))