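; BP_GeometryTrace is an actor that demonstrates box, capsule and sphere shape traces, drawing each for debugging.
; Every Tick, a Sequence runs the three traces on the Visibility channel with one-frame debug draw and leaves the results unused.
; Their starts are staggered along X from the actor's location, but all three converge on the same end point along +Y.
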(event EventBeginPlay)

(event Collision|EventActorBeginOverlap
  (params (OtherActor :type Actor%20Object%20Reference)))

(event EventTick
  (params (DeltaSeconds :type Float%20%28single-precision%29))
  (bind _returnvalue (Transformation|GetActorLocation))
  (bind _returnvalue_2 (Transformation|GetActorLocation))
  (bind _returnvalue_3 (Transformation|GetActorLocation))
  (Utilities|FlowControl|Sequence
    (:then_0
      (Collision|BoxTraceByChannel _returnvalue_2 (+ _returnvalue_2 "0.000000,500.000000,0.000000") "15.000000,15.000000,15.000000" "0, 0, 0" "TraceTypeQuery1" false 0 "ForOneFrame"))
    (:then_1
      (Collision|CapsuleTraceByChannel (+ _returnvalue_3 "200.000000,0.000000,0.000000") (+ _returnvalue_3 "0.000000,500.000000,0.000000") 15.0 5e+01 "TraceTypeQuery1" false 0 "ForOneFrame"))
    (:then_2
      (Collision|SphereTraceByChannel (+ _returnvalue "400.000000,0.000000,0.000000") (+ _returnvalue "0.000000,500.000000,0.000000") 15.0 "TraceTypeQuery1" false 0 "ForOneFrame"))))

(fn ConstructionScript)